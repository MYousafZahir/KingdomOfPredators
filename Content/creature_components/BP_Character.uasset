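; Creature Character Blueprint that tracks pawn sightings and can emit noise while moving.
; BeginPlay caches the BP_Stork actor, and PawnSensing raises SeesPawn, which a retriggerable delay clears shortly after the last sighting.
; MakeNoiseOnMovement uses a countdown to throttle zero-loudness noise events and camera shutter sounds while velocity is non-zero, but nothing in this graph calls it and Tick is empty.
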(event `self.ReceiveBeginPlay`
  (bind _returnvalue (`GameplayStatics.GetActorOfClass` "/Game/creature_components/BP_Stork.BP_Stork_C"))
  (set `self.Stork` _returnvalue)
  (set `self.SeesPawn` false))

(event `self.ReceiveTick`
  (params (DeltaSeconds :type "Float (single-precision)")))

(event `self.PawnSensing.OnSeePawn`
  (params (Pawn :type "Pawn Object Reference"))
  (set `self.SeesPawn` true)
  (`KismetSystemLibrary.RetriggerableDelay` 0.6)
  (set `self.SeesPawn` false))

(fn `MakeNoiseOnMovement`
  (bind _returnvalue (`self.K2_GetActorLocation`))
  (bind _emittime (`self.emitTime`))
  (if (and (<= _emittime 0.0) (not (`KismetMathLibrary.Vector_IsZero` (`self.GetVelocity`))))
    (`PawnNoiseEmitterComponent.MakeNoise` (`self.PawnNoiseEmitter`) null 0.0 _returnvalue)
    (`GameplayStatics.PlaySoundAtLocation` "/Engine/VREditor/Sounds/UI/Camera_Shutter.Camera_Shutter" _returnvalue (struct) 1.0 1.0 0.0 null null null null)
    (set `self.emitTime` 1.0)
    (else
      (set `self.emitTime` (- _emittime (`GameplayStatics.GetWorldDeltaSeconds`))))))

(fn `UserConstructionScript`)